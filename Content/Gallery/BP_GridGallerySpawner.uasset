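; BP_GridGallerySpawner computes slot transforms for a gallery grid, though it spawns nothing itself.
; InitGrid rebuilds LocationArray from Rows and Cols, stepping along Y and down Z from the actor's truncated location at fixed spacing, with X at zero.
; CalcRows and CalcColumns sketch a square-root-based near-square layout, but their item count is zero and InitGrid does not call them.
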(event `Init Grid`
  (bind _y (.y (.location (`self.GetTransform`))))
  (set `self.Location_Array` (`|MakeArray`))
  (set `self.y-coord` (`KismetMathLibrary.FTrunc` _y))
  (set `self.z-coord` (`KismetMathLibrary.FTrunc` (.z (.location (`self.GetTransform`)))))
  (for _ (range 1 (+ (`self.Rows`) 1))
    (for _ (range (`self.Cols`))
      (`KismetArrayLibrary.Array_Add` (`self.Location_Array`) (`KismetMathLibrary.MakeTransform` (`KismetMathLibrary.MakeVector` 0.0 (`KismetMathLibrary.Conv_IntToDouble` (`self.y-coord`)) (`KismetMathLibrary.Conv_IntToDouble` (`self.z-coord`)))))
      (set `self.y-coord` (+ (`self.y-coord`) 550)))
    (set `self.z-coord` (- (`self.z-coord`) 320))
    (set `self.y-coord` (`KismetMathLibrary.FTrunc` _y))))

(fn `Calc Columns`
  (params (rows :type Integer))
  (returns (Columns :type Integer))
  (return (`KismetMathLibrary.FCeil` (`KismetMathLibrary.SafeDivide` (`KismetMathLibrary.Conv_IntToDouble` 0) (`KismetMathLibrary.Conv_IntToDouble` rows)))))

(fn `Calc Rows`
  (returns (rows :type Integer))
  (return (`KismetMathLibrary.FFloor` (`KismetMathLibrary.Sqrt` (`KismetMathLibrary.Conv_IntToDouble` 0)))))

(fn `UserConstructionScript`
  (`KismetSystemLibrary.PrintString` "*** BP_Grid Construction***" false))